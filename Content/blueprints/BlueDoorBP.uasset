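; BlueDoorBP is a locked door that opens only for a third-person character carrying the blue key.
; When that character overlaps the Box trigger and HasBlueKey is true, it plays the open-door sound and a Timeline swings the mesh's yaw up to 120 degrees, scaled by its track.
; Without the key, it creates a FindBlueKey widget for the player's controller and adds it to the viewport.
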(event `self.Box.OnComponentBeginOverlap`
  (params (OverlappedComponent :type "PrimitiveComponent Object Reference") (OtherActor :type "Actor Object Reference") (OtherComp :type "PrimitiveComponent Object Reference") (OtherBodyIndex :type Integer) (bFromSweep :type Boolean) (SweepResult :type "HitResult Structure (by ref)"))
  (bind _ascharacter (cast `Character` OtherActor))
  (bind _asthird_person_character (cast `/Game/ThirdPersonBP/Blueprints/ThirdPersonCharacter` _ascharacter))
  (if (`/Game/ThirdPersonBP/Blueprints/ThirdPersonCharacter.HasBlueKey` _asthird_person_character)
    (`GameplayStatics.PlaySoundAtLocation` "/Game/blueprints/soundeffects/Opendoor_cue.Opendoor_cue" (`self.K2_GetActorLocation` OtherActor) (struct) 1.0 1.0 0.0 null null null)
    (bind (_direction _newtrack_0) (`Timeline|Timeline_0`)
      (:`Update`
        (`SceneComponent.K2_SetRelativeRotation` (`self.StaticMesh`) (`KismetMathLibrary.MakeRotator` 0.0 0.0 (* _newtrack_0 120.0)) false false)))
    (else
      (bind _asplayer_controller (cast `PlayerController` (`Pawn.GetController` _asthird_person_character)))
      (bind _returnvalue (`|CreateWidget` "/Game/Maps/Menu/Widgets/FindBlueKey.FindBlueKey_C" _asplayer_controller))
      (`UserWidget.AddToViewport` _returnvalue 0))))

(fn `UserConstructionScript`)