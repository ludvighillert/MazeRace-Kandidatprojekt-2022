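; Procedural maze actor that builds a seeded grid maze in the Construction Script, placing a MazeGround instance on each path tile.
; GenerateMaze runs a randomized depth-first backtracker: AddneighbourLoc recursively carves two-tile steps from a random start, and BackTrack pops pending cells, adding bridge tiles to the path.
; Dead ends are collected but unused, and wall instancing is disconnected.
; A Placeplayerstart event moves the ThirdPersonCharacter to a fixed location.
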(event `self.MazeGround.OnComponentHit`
  (params (HitComponent :type "PrimitiveComponent Object Reference") (OtherActor :type "Actor Object Reference") (OtherComp :type "PrimitiveComponent Object Reference") (NormalImpulse :type "Vector Structure") (Hit :type "HitResult Structure (by ref)")))

(event `Place player start`
  (bind _outactors (`GameplayStatics.GetAllActorsOfClass` "/Game/ThirdPersonBP/Blueprints/ThirdPersonCharacter.ThirdPersonCharacter_C"))
  (bind (_sweephitresult _returnvalue) (`self.K2_SetActorLocation` (`|GetArrayItem` _outactors) (0.0 0.0 -50.0) false false))
  (`KismetSystemLibrary.PrintString` (`KismetStringLibrary.Conv_BoolToString` _returnvalue)))

(fn `AddneighbourLoc`
  (params (Size :type "IntPoint Structure (by ref)") (RandStream :type "RandomStream Structure (by ref)") (`Current Loc` :type "IntPoint Structure (by ref)") (`Path Location` :type "Set of IntPoint Structure (by ref)") (`bridge tiles` :type "Set of IntPoint Structure (by ref)") (`to check` :type "Set of IntPoint Structure (by ref)") (`End paths` :type "Set of IntPoint Structure (by ref)"))
  (locals (NeighbourIndex :type Integer))
  (bind _returnvalue (+ (`local.NeighbourIndex`) 1))
  (bind (_floor _bridge) (`self.GetNeighbourAndBridge` (`local.Current Loc`) (`local.NeighbourIndex`)))
  (set `local.NeighbourIndex` (`KismetMathLibrary.RandomIntegerInRangeFromStream` 0 3 (`local.RandStream`)))
  (if (`self.CheckifvalidLoc` (`self.GetNeighbourAndBridge` (`local.Current Loc`) (`local.NeighbourIndex`)) (`self.Size`) (`local.Path Location`) (`local.bridge tiles`)) :!label _label
    (`BlueprintSetLibrary.Set_Add` (`local.Path Location`) _floor)
    (`BlueprintSetLibrary.Set_Add` (`local.bridge tiles`) _bridge)
    (`BlueprintSetLibrary.Set_Add` (`local.to check`) _floor)
    (`self.AddneighbourLoc` (`self.Size`) (`local.RandStream`) _floor (`local.Path Location`) (`local.bridge tiles`) (`local.to check`) (`local.End paths`))
    (else
      (`/Game/blueprints/CostumemacroLib.DoN+` 4
        (:`Exit`
          (set `local.NeighbourIndex` (`KismetMathLibrary.SelectInt` 0 _returnvalue (>= _returnvalue 4)))
          (goto _label))
        (:`OverNth`
          (bind _counter1 (`self.GetNeighbourCount` (`local.Current Loc`) (`local.Path Location`)))
          (if (== _counter1 1)
            (`BlueprintSetLibrary.Set_Add` (`local.End paths`) (`local.Current Loc`))))))))

(fn `BackTrack`
  (params (`Current tile` :type "IntPoint Structure (by ref)") (`to check` :type "Set of IntPoint Structure (by ref)") (`Bridge tiles` :type "Set of IntPoint Structure (by ref)") (`Path Location` :type "Set of IntPoint Structure (by ref)"))
  (bind _result (`BlueprintSetLibrary.Set_ToArray` `to check`))
  (bind _output (`|GetArrayItem` _result (`KismetArrayLibrary.Array_LastIndex` _result)))
  (`|VariableSetRef` (`local.Current tile`) _output)
  (`BlueprintSetLibrary.Set_Remove` (`local.to check`) _output)
  (bind _result_2 (`BlueprintSetLibrary.Set_ToArray` (`local.Bridge tiles`)))
  (bind _output_2 (`|GetArrayItem` _result_2 (`KismetArrayLibrary.Array_LastIndex` _result_2)))
  (`BlueprintSetLibrary.Set_Add` (`local.Path Location`) _output_2)
  (`BlueprintSetLibrary.Set_Remove` (`local.Bridge tiles`) _output_2))

(fn `Generate Maze`
  (params (Seed :type Integer :default 1) (Size :type "IntPoint Structure"))
  (returns (`Path locationOut` :type "Set of IntPoint Structure") (`End PathsOut` :type "Set of IntPoint Structure") (L_Size1 :type "IntPoint Structure"))
  (locals (RandStream :type "RandomStream Structure") (L_Size :type "IntPoint Structure") (StartingLoc :type "IntPoint Structure") (CurrentLoc :type "IntPoint Structure") (`Path location` :type "Set of IntPoint Structure") (BridgeTiles :type "Set of IntPoint Structure") (toCheck :type "Set of IntPoint Structure") (`End Paths` :type "Set of IntPoint Structure"))
  (`KismetMathLibrary.SetRandomStreamSeed` (`local.RandStream`) Seed)
  (set `local.L_Size` Size)
  (bind _output_get (set `local.StartingLoc` (`self.GetRandlocinBounds` (`local.L_Size`) (`local.RandStream`))))
  (set `local.CurrentLoc` _output_get)
  (`self.AddneighbourLoc` (`local.L_Size`) (`local.RandStream`) (`local.CurrentLoc`) (`local.Path location`) (`local.BridgeTiles`) (`local.toCheck`) (`local.End Paths`) :!label _label)
  (if (> (`BlueprintSetLibrary.Set_Length` (`local.toCheck`)) 0)
    (`self.BackTrack` (`local.CurrentLoc`) (`local.toCheck`) (`local.BridgeTiles`) (`local.Path location`))
    (goto _label)
    (else
      (return (`local.Path location`) (`local.End Paths`) (`local.L_Size`)))))

(fn `GetNeighbourCount`
  (params (CurrentLoc :type "IntPoint Structure") (PathLocation :type "Set of IntPoint Structure (by ref)"))
  (returns (counter1 :type Integer))
  (locals (counter :type Integer))
  (for _array_element (`self.Getneighbourloc` CurrentLoc)
    (if (`BlueprintSetLibrary.Set_Contains` (`local.PathLocation`) _array_element)
      (`/Engine/EditorBlueprintResources/StandardMacros.IncrementInt` (`local.counter`))))
  (return (`local.counter`)))

(fn `UserConstructionScript`
  (bind _tilesize (`self.TileSize`))
  (bind (_path_locationout _end_pathsout _l_size1) (`self.Generate Maze` (`self.Seed`) (`self.Size`)))
  (bind _result (`BlueprintSetLibrary.Set_ToArray` _path_locationout))
  (for _array_element _result
    (bind (_x _y) (break `IntPoint` _array_element))
    (`InstancedStaticMeshComponent.AddInstance` (`self.MazeGround`) (`KismetMathLibrary.MakeTransform` (`KismetMathLibrary.MakeVector` (* _x _tilesize) (* _y _tilesize))))))